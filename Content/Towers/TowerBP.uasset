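; Tower actor that automatically fires projectiles at AIRunner enemies in range, with mesh and stats loaded from the hard-coded "Chair" row of TowerDataTable.
; A range-sized sphere acquires a runner on overlap when idle and drops it on exit.
; Without a target, Tick runs a delay-throttled sphere trace to pick the closest runner.
; With one, it spawns projectiles carrying target and damage, using FireRate as the reload delay.
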(event `CheckForNewTarget`
  (bind _returnvalue (`self.K2_GetActorLocation`))
  (set `self.CheckForTarget` true)
  (bind (_outhits _returnvalue_2) (`KismetSystemLibrary.SphereTraceMultiForObjects` _returnvalue (- _returnvalue (0.0 0.0 1.0)) (`.Range_7_6B55B12741651B3EE0BF3BA19CE43B3D` (break `/Game/Towers/TowerStruct` (`self.TowerStruct`))) (`|MakeArray` "ObjectTypeQuery3" :!type "EObjectTypeQuery Enum")))
  (if _returnvalue_2
    (bind _target (`self.ClosestTargetCalculation` _outhits))
    (`/Engine/EditorBlueprintResources/StandardMacros.IsValid` _target
      (:`Is Valid`
        (set `self.TowerTarget` _target))
      (:`Is Not Valid`
        _)))
  (`KismetSystemLibrary.Delay` 0.2)
  (set `self.CheckForTarget` false))

(event `Shoot`
  (bind (_name _damage _range _firerate) (break `/Game/Towers/TowerStruct` (`self.TowerStruct`)))
  (set `self.Reload` true)
  (`|SpawnActorFromClass` "/Game/Towers/TowerProjectile.TowerProjectile_C" (`self.GetTransform`) "AlwaysSpawn" "OverrideRootScale" null (`self.TowerTarget`) _damage null)
  (`KismetSystemLibrary.Delay` _firerate)
  (set `self.Reload` false))

(event `self.ReceiveTick`
  (params (DeltaSeconds :type "Float (single-precision)"))
  (`/Engine/EditorBlueprintResources/StandardMacros.IsValid` (`self.TowerTarget`)
    (:`Is Valid`
      (if (not (`self.Reload`))
        (`self.Shoot`)))
    (:`Is Not Valid`
      (if (not (`self.CheckForTarget`))
        (`self.CheckForNewTarget`)))))

(event `self.Sphere.OnComponentBeginOverlap`
  (params (OverlappedComponent :type "PrimitiveComponent Object Reference") (OtherActor :type "Actor Object Reference") (OtherComp :type "PrimitiveComponent Object Reference") (OtherBodyIndex :type Integer) (bFromSweep :type Boolean) (SweepResult :type "HitResult Structure (by ref)"))
  (`/Engine/EditorBlueprintResources/StandardMacros.IsValid` (`self.TowerTarget`)
    (:`Is Not Valid`
      (bind _asairunner (cast `/Game/AI/AIRunner` OtherActor))
      (set `self.TowerTarget` _asairunner))))

(event `self.Sphere.OnComponentEndOverlap`
  (params (OverlappedComponent :type "PrimitiveComponent Object Reference") (OtherActor :type "Actor Object Reference") (OtherComp :type "PrimitiveComponent Object Reference") (OtherBodyIndex :type Integer))
  (if (== (`self.TowerTarget`) OtherActor)
    (set `self.TowerTarget` null)))

(event `self.ReceiveBeginPlay`
  (bind _returnvalue (`|GetDataTableRow` "/Game/Towers/TowerDataTable.TowerDataTable" "Chair")
    (:`then`
      (set `self.TowerStruct` _returnvalue)
      (`self.TowerInit`))))

(event `TowerInit`
  (bind (_name _damage _range _firerate _mesh) (break `/Game/Towers/TowerStruct` (`self.TowerStruct`)))
  (`StaticMeshComponent.SetStaticMesh` (`self.TowerMesh`) _mesh)
  (`SphereComponent.SetSphereRadius` (`self.Sphere`) _range true))

(fn `ClosestTargetCalculation`
  (params (HitResults :type "Array of HitResult Structure"))
  (returns (Target :type "/Game/AI/AIRunner Object Reference"))
  (locals (TempTarget :type "/Game/AI/AIRunner Object Reference") (TempDistance :type "Float (double-precision)" :default 0.0))
  (for _array_element HitResults
    (bind (_bblockinghit _binitialoverlap _time _distance _location _impactpoint _normal _impactnormal _physmat _hitactor) (`GameplayStatics.BreakHitResult` _array_element))
    (bind _asairunner (cast `/Game/AI/AIRunner` _hitactor))
    (`/Engine/EditorBlueprintResources/StandardMacros.IsValid` (`local.TempTarget`)
      (:`Is Valid`
        (bind _returnvalue (`KismetMathLibrary.VSize` (- (`self.K2_GetActorLocation`) (`self.K2_GetActorLocation` _hitactor))))
        (if (< _returnvalue (`local.TempDistance`))
          (set `local.TempTarget` _asairunner)
          (set `local.TempDistance` _returnvalue)))
      (:`Is Not Valid`
        (set `local.TempTarget` _asairunner)
        (set `local.TempDistance` _returnvalue))))
  (return (`local.TempTarget`)))

(fn `UserConstructionScript`)