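; Auto-turret actor that targets the nearest pawn within sensing range and line of sight, then shoots projectiles at it.
; Each tick it picks a target, turns its top at constant speed with clamped pitch, and fires once cooled down and a dot-product check confirms aim.
; A looping DoN with delays alternates left and right barrels for two rounds per burst, starting a curve-driven recoil timeline with each shot.
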(event `self.ReceiveBeginPlay`
  (`TimelineComponent.SetFloatCurve` (`self.RecoilTimelineL`) "/Game/Turret/RecoilCurve.RecoilCurve" "Recoil")
  (`TimelineComponent.SetFloatCurve` (`self.RecoilTimelineR`) "/Game/Turret/RecoilCurve.RecoilCurve" "Recoil"))

(event `self.ReceiveTick`
  (params (DeltaSeconds :type "Float (single-precision)"))
  (`self.findBestTarget`)
  (`self.Target`
    (:`then`
      (`self.UpdateTurretRotation` DeltaSeconds)
      (`self.UpdateFire`))
    (:`else`)))

(event `fire`
  (set `self.TimeOfLastFire` (`KismetSystemLibrary.GetGameTimeInSeconds`))
  (`|ExecutionSequence`
    (:`then_0`
      (goto _label :!via `Reset`))
    (:`then_1`
      (`/Engine/EditorBlueprintResources/StandardMacros.Do N` 2 :!label _label
        (:`Exit`
          (`|SpawnActorFromClass` "/Game/FirstPersonBP/Blueprints/FirstPersonProjectile.FirstPersonProjectile_C" (`SceneComponent.GetSocketTransform` (`self.StaticMeshBarrelL`) "FireSocket" "RTS_World") "Undefined" "OverrideRootScale" null null)
          (`TimelineComponent.PlayFromStart` (`self.RecoilTimelineL`))
          (`KismetSystemLibrary.Delay` 0.2)
          (`|SpawnActorFromClass` "/Game/FirstPersonBP/Blueprints/FirstPersonProjectile.FirstPersonProjectile_C" (`SceneComponent.GetSocketTransform` (`self.StaticMeshBarrelR`) "FireSocket" "RTS_World") "Undefined" "OverrideRootScale" null null)
          (`TimelineComponent.PlayFromStart` (`self.RecoilTimelineR`))
          (`KismetSystemLibrary.Delay` 0.2)
          (goto _label))))))

(fn `findBestTarget`
  (locals (`BestDistance (local)` :type "Float (double-precision)") (`CurrentDistance (local)` :type "Float (double-precision)") (`BestTarget (local)` :type "Actor Object Reference") (`CurrentTarget (local)` :type "Actor Object Reference"))
  (set `local.BestDistance (local)` (+ (`self.SensingRange`) 1.0))
  (bind _outactors (`KismetSystemLibrary.SphereOverlapActors` (`self.K2_GetActorLocation`) (`self.SensingRange`) (`|MakeArray` "ObjectTypeQuery3" :!type "EObjectTypeQuery Enum") "/Script/Engine.Actor"))
  (for _array_element _outactors
    (bind _output_get (set `local.CurrentTarget (local)` _array_element))
    (bind _output_get_2 (set `local.CurrentDistance (local)` (`self.GetDistanceTo` _output_get self)))
    (if (or (< _output_get_2 (`local.BestDistance (local)`)) (not (`KismetSystemLibrary.IsValid` (`local.BestTarget (local)`))))
      (bind _result (`/Game/MyFunctionLibrary.HasLineOfSight` (`SceneComponent.K2_GetComponentLocation` (`self.StaticMeshTop`)) (`self.K2_GetActorLocation` (`local.CurrentTarget (local)`)) (`|MakeArray` self (`local.CurrentTarget (local)`) :!type "Actor Object Reference")))
      (if _result
        (set `local.BestTarget (local)` (`local.CurrentTarget (local)`))
        (set `local.BestDistance (local)` (`local.CurrentDistance (local)`)))))
  (set `self.Target` (`local.BestTarget (local)`)))

(fn `UpdateFire`
  (if (> (- (`KismetSystemLibrary.GetGameTimeInSeconds`) (`self.TimeOfLastFire`)) (`self.RateOfFire`))
    (if (> (`KismetMathLibrary.Dot_VectorVector` (`KismetMathLibrary.GetDirectionUnitVector` (`SceneComponent.K2_GetComponentLocation` (`self.StaticMeshTop`)) (`self.K2_GetActorLocation` (`self.Target`))) (`SceneComponent.GetForwardVector` (`self.StaticMeshTop`))) 0.99)
      (`self.fire`))))

(fn `UpdateTurretRotation`
  (params (DeltaSeconds :type "Float (double-precision)"))
  (locals (NewRotation :type "Rotator Structure" :default (struct)) (NewLocalVar_1 :type "Rotator Structure" :default (struct)))
  (bind _output_get (set `local.NewLocalVar_1` (`KismetMathLibrary.RInterpTo_Constant` (`SceneComponent.K2_GetComponentRotation` (`self.StaticMeshTop`)) (`KismetMathLibrary.FindLookAtRotation` (`SceneComponent.K2_GetComponentLocation` (`self.StaticMeshTop`)) (`self.K2_GetActorLocation` (`self.Target`))) (`local.DeltaSeconds`) (`self.RotationSpeed`))))
  (`SceneComponent.K2_SetWorldRotation` (`self.StaticMeshTop`) (`KismetMathLibrary.MakeRotator` (.roll _output_get) (`KismetMathLibrary.ClampAngle` (.pitch _output_get) -45.0 75.0) (.yaw _output_get)) false false))

(fn `UserConstructionScript`)